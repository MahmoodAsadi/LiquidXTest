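; BP_Lap is a ceiling lamp that toggles on and off when interacted with.
; BeginPlay creates a dynamic material instance on the lamp mesh and stores it.
; The OnInteractBody event flips the On state, sets the point light's visibility to match and switches the material's Glow parameter so the mesh glows only while lit.
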(event EventOnInteractBody
  (params (FromActor :type Actor%20Object%20Reference))
  (Variables|Default|SetOn (not (Variables|Default|GetOn)))
  (Rendering|SetVisibility (Variables|Default|GetPointLight) (Variables|Default|GetOn) false)
  (Rendering|Material|SetScalarParameterValue (Variables|Default|GetLamp%20DMI) "Glow" (Math|Float|SelectFloat 5.0 0.0 (Variables|Default|GetOn)) :!class /Script/Engine.MaterialInstanceDynamic))

(event EventBeginPlay
  (bind _returnvalue (Rendering|Material|CreateDynamicMaterialInstance (Variables|Default|GetSM_Lamp_Ceiling) 0 0 "None" :!class /Script/Engine.PrimitiveComponent))
  (Variables|Default|SetLamp%20DMI _returnvalue))

(fn ConstructionScript)